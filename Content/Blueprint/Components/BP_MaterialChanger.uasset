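; BP_MaterialChanger is an actor component that switches its owner's static meshes between an on material and an off material.
; Toggle flips the boolean State and SetState assigns it directly, and both then call HandleMaterials to pick MaterialOn or MaterialOff.
; SetMaterial applies the chosen material at MaterialIndex to every StaticMeshComponent on the owning actor.
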(fn `HandleMaterials`
  (returns (State :type Boolean))
  (bind _state (`self.State`))
  (if _state
    (`self.SetMaterial` (`self.MaterialOn`) (`self.MaterialIndex`))
    (return _state)
    (else
      (`self.SetMaterial` (`self. MaterialOff`) (`self.MaterialIndex`)))))

(fn `SetMaterial`
  (params (Material :type "MaterialInterface Object Reference") (Index :type Integer))
  (for _array_element (`Actor.K2_GetComponentsByClass` (`self.GetOwner` self) "/Script/Engine.StaticMeshComponent")
    (`PrimitiveComponent.SetMaterial` _array_element Index Material)))

(fn `SetState`
  (params (NewState :type Boolean))
  (set `self.State` NewState)
  (`self.HandleMaterials`))

(fn `Toggle`
  (set `self.State` (not (`self.State`)))
  (`self.HandleMaterials`))