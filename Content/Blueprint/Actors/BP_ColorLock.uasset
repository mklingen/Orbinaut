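; BP_ColorLock is an actor that visually reflects whether its Lock is locked.
; On BeginPlay it binds to the Lock's OnLockStateChanged event and passes the current IsLocked value to BPMaterialChanger.
; Each later lock state change forwards the new value to BPMaterialChanger's SetState, so the material follows the lock without using Tick.
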(event `self.ReceiveBeginPlay`
  (bind _lock (`self.Lock`))
  (`parent.ReceiveBeginPlay`)
  (add `LockComponent.OnLockStateChanged` _lock (delegate `OnLockStatechanged`))
  (`/Game/Blueprint/Components/BP_MaterialChanger.SetState` (`self.BP_MaterialChanger`) (`LockComponent.IsLocked` _lock)))

(event `OnLockStatechanged`
  (params (Lock :type "LockComponent Object Reference") (Key :type "KeyComponent Object Reference") (IsLocked :type Boolean))
  (`/Game/Blueprint/Components/BP_MaterialChanger.SetState` (`self.BP_MaterialChanger`) IsLocked))

(fn `UserConstructionScript`
  (`parent.UserConstructionScript`))