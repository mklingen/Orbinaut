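; BP_ExitPortal is an exit portal actor that shows its open or closed state through the material on its static mesh.
; On BeginPlay it binds handlers to player overlap, opened and closed events.
; Player overlap and opened share one handler that applies the open material, while closed applies the closed material.
; The graph only swaps materials and contains no exit or level transition logic.
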(event `self.ReceiveBeginPlay`
  (add `self.OnPlayerOverlap` self (delegate `OnPlayerOverlapped`))
  (add `self.OnOpened` self (delegate `OnPlayerOverlapped`))
  (add `self.OnClosed` self (delegate `OnPortalClosed`)))

(event `OnPlayerOverlapped`
  (`PrimitiveComponent.SetMaterial` (`self.StaticMesh`) 0 (`self.OpenMaterial`)))

(event `OnPortalClosed`
  (`PrimitiveComponent.SetMaterial` (`self.StaticMesh`) 0 (`self.ClosedMaterial`)))

(fn `UserConstructionScript`)